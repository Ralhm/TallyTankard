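; Player Blueprint for a rhythm drinking game played with a gyroscope tankard read over the game mode's serial port.
; Debug inputs read and parse the gyro string, and Tick draws debug lines for the tankard's rotation.
; Slam input passes the game mode's beat state to its alcohol update and fires booze VFX on beat.
; DrinkCheck detects tipping by comparing the tilted up vector's dot with world up against a threshold.
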(event EventBeginPlay)

(event EventTick
  (params (DeltaSeconds :type Float%20%28single-precision%29))
  (CallFunction|DebugRotationCheck))

(event Collision|EventActorBeginOverlap
  (params (OtherActor :type Actor%20Object%20Reference)))

(event Input|ActionEvents|InputActionCheckGyroscope
  (params (Key :type Key%20Structure :default "None"))
  (:Pressed
    (CallFunction|ReadGyroscope)))

(event Input|ActionEvents|InputActionCheckRotation
  (params (Key :type Key%20Structure :default "None"))
  (:Pressed
    (CallFunction|ReadGyroscope)))

(event Input|ActionEvents|InputActionSlam
  (params (Key :type Key%20Structure :default "None"))
  (:Pressed
    (CallFunction|SlamBeatCheck)))

(fn ConstructionScript)

(fn ReadGyroscope
  ;[1 1 1] DEBUG
  (bind _asbp_game_mode (Utilities|Casting|CastToBP_GameMode (Game|GetGameMode)))
  (bind _returnvalue (Class|SerialCom|ReadString (Variables|/Game/Blueprints/BP_GameMode.BP_GameMode_C|GetSerial%20Port _asbp_game_mode)))
  (bind _output_get (Variables|Default|SetGyroString _returnvalue))
  (Class|TallyTankardPlayer|ParseGyroString))

(fn RaiseBeatCheck
  (bind _returnvalue (Class|TallyTankardPlayer|RaiseTankard))
  (return _returnvalue))

(fn SlamBeatCheck
  (bind _gamemode (Variables|Default|GetGameMode))
  (bind _inbeat (Variables|/Script/TallyTankard.TallyTankardGameMode|GetinBeat _gamemode))
  (bind _asbp_game_mode (Utilities|Casting|CastToBP_GameMode _gamemode))
  (Default|UpdateAlcohol _asbp_game_mode _inbeat)
  (if _inbeat
    (Class|NiagaraSystemWidget|ActivateSystem (Variables|/Game/Widgets/BeatWidget.BeatWidget_C|GetBoozeVFX (Variables|/Game/Blueprints/BP_GameMode.BP_GameMode_C|GetBeatWidget _asbp_game_mode)) true))
  (return _inbeat))

(fn DrinkCheck
  (bind _returnvalue (Math|Vector|VectorUp))
  (bind _drinkthreshold (Variables|Default|GetDrinkThreshold))
  (bind _xangle (Variables|Default|GetxAngle))
  (bind _yangle (Variables|Default|GetyAngle))
  (bind _zangle (Variables|Default|GetzAngle))
  (bind _returnvalue_2 (Math|Rotator|MakeRotator _xangle _yangle _zangle))
  (bind _returnvalue_3 (Math|Vector|GetUpVector _returnvalue_2))
  (bind _returnvalue_4 (Math|Vector|DotProduct _returnvalue_3 _returnvalue))
  (bind _returnvalue_5 (< _returnvalue_4 _drinkthreshold))
  ;[1 1 1] Returns True if angled sideways
  ;;[1 1 1] Debug Visualizer
  (Transformation|SetWorldRotation (Variables|Default|GetDebugCylinder) _returnvalue_2 false false)
  (Development|PrintString (Utilities|String|ToString(Boolean) _returnvalue_5) true true "(R=0.000000,G=0.000000,B=0.000000,A=1.000000)")
  (return _returnvalue_5))

(fn DebugRotationCheck
  (bind _debugcylinder (Variables|Default|GetDebugCylinder))
  (bind _debugcylinder_2 (Variables|Default|GetDebugCylinder))
  (bind _returnvalue (Transformation|GetWorldLocation _debugcylinder_2))
  (bind _returnvalue_2 (Transformation|GetWorldLocation _debugcylinder))
  ;[1 1 1] Draw a cylinder to the screen to track the tankards rotation DEBUG
  (Rendering|Debug|DrawDebugLine :LineStart _returnvalue_2 :LineEnd (+ _returnvalue_2 (* (Math|Vector|GetUpVector _debugcylinder) 2e+02)) :Duration 0.1 :Thickness 5.0)
  (Rendering|Debug|DrawDebugLine _returnvalue (+ _returnvalue (* (Math|Vector|GetUpVector (Math|Rotator|MakeRotator (Variables|Default|GetxAngle) (Variables|Default|GetyAngle) (Variables|Default|GetzAngle))) 3e+02)) "(R=0.000000,G=0.994792,B=0.046272,A=1.000000)" 0.1 5.0))